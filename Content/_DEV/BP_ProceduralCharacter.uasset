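; Player character Blueprint with crouch, sprint, slide, vault and mantle moves, switchable first and third-person cameras, slow motion and a procedural IK toggle.
; Timelines blend capsule height, mesh offset, crouch boom length and sprint FOV, with an overhead trace blocking stand-up.
; Vaulting traces obstacle height, depth and landing spot, then plays a motion-warped montage in Flying mode without capsule collision.
; Jump defers to MantleSystem's ground check before jumping normally.
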(event Input|EnhancedActionEvents|EnhancedInputActionIA_IKSwitch
  (params (ActionValue :type Boolean) (ElapsedSeconds :type Float%20%28double-precision%29) (TriggeredSeconds :type Float%20%28double-precision%29) (InputAction :type Input%20Action%20Object%20Reference :default "/Game/ThirdPerson/Input/Actions/IA_IKSwitch.IA_IKSwitch"))
  (:Started
    (Utilities|FlowControl|FlipFlop
      (:A
        (Variables|Default|SetIK_ON true)
        (bind _aswbp_overhead_text (Utilities|Casting|CastToWBP_OverheadText (UserInterface|GetUserWidgetObject (Variables|Default|GetOverheadTextWidget))))
        (Variables|/Game/_DEV/UI/WBP_OverheadText.WBP_OverheadText_C|Settexting _aswbp_overhead_text "PROCEDURAL IK : ON"))
      (:B
        (Variables|Default|SetIK_ON false)
        (bind _aswbp_overhead_text_2 (Utilities|Casting|CastToWBP_OverheadText (UserInterface|GetUserWidgetObject (Variables|Default|GetOverheadTextWidget))))
        (Variables|/Game/_DEV/UI/WBP_OverheadText.WBP_OverheadText_C|Settexting _aswbp_overhead_text_2 "PROCEDURAL IK : OFF")))))

(event Input|EnhancedActionEvents|EnhancedInputActionIA_Sprint
  (params (ActionValue :type Boolean) (ElapsedSeconds :type Float%20%28double-precision%29) (TriggeredSeconds :type Float%20%28double-precision%29) (InputAction :type Input%20Action%20Object%20Reference :default "/Game/ThirdPerson/Input/Actions/IA_Sprint.IA_Sprint"))
  (bind _charactermovement (Variables|Character|GetCharacterMovement))
  (:Triggered
    ;[1 1 1] Sprint
    (if (> (Math|Vector|VectorLength (Variables|/Script/Engine.MovementComponent|GetVelocity (Variables|Character|GetCharacterMovement))) 0.0)
      (Variables|Default|SetSprinting true)
      (Variables|/Script/Engine.CharacterMovementComponent|SetMaxWalkSpeed _charactermovement 7e+02)
      (if (AI|Components|NavMovement|IsMovingonGround (Variables|Character|GetCharacterMovement))
        (bind _time (Timeline|CameraFOV Play)
          (:Update
            (Camera|SetFieldOfView (Variables|Default|GetCombatCamera) (Math|Float|Lerp 9e+01 105.0 _time))
            (Camera|SetFieldOfView (Variables|Default|GetFollowCamera) (Math|Float|Lerp 8e+01 9e+01 _time))
            (Camera|SetFieldOfView (Variables|Default|GetFPSCamera) (Math|Float|Lerp 1e+02 1.2e+02 _time)))))))
  (:Completed
    (if (> (Math|Vector|VectorLength (Variables|/Script/Engine.MovementComponent|GetVelocity (Variables|Character|GetCharacterMovement))) 0.0)
      (Variables|Default|SetSprinting false)
      (Variables|/Script/Engine.CharacterMovementComponent|SetMaxWalkSpeed _charactermovement 2e+02)
      (if (AI|Components|NavMovement|IsMovingonGround (Variables|Character|GetCharacterMovement))
        (Timeline|CameraFOV Reverse)))))

(event Input|EnhancedActionEvents|EnhancedInputActionIA_SlowMotion
  (params (ActionValue :type Boolean) (ElapsedSeconds :type Float%20%28double-precision%29) (TriggeredSeconds :type Float%20%28double-precision%29) (InputAction :type Input%20Action%20Object%20Reference :default "/Game/ThirdPerson/Input/Actions/IA_SlowMotion.IA_SlowMotion"))
  ;[1 1 1] SlowMotion
  (:Started
    (Utilities|FlowControl|FlipFlop
      (:A
        (Utilities|Time|SetGlobalTimeDilation 0.35))
      (:B
        (Utilities|Time|SetGlobalTimeDilation 1.0)))))

(event Input|EnhancedActionEvents|EnhancedInputActionIA_Crouch
  (params (ActionValue :type Boolean) (ElapsedSeconds :type Float%20%28double-precision%29) (TriggeredSeconds :type Float%20%28double-precision%29) (InputAction :type Input%20Action%20Object%20Reference :default "/Game/ThirdPerson/Input/Actions/IA_Crouch.IA_Crouch"))
  (bind _returnvalue (Transformation|GetActorLocation))
  (bind _charactermovement (Variables|Character|GetCharacterMovement))
  ;[1 1 1] Crouch
  (:Started
    (if (and (not (Variables|Default|GetCrouched)) (not (Variables|Default|GetSprinting)))
      (Variables|Default|SetCrouched true)
      (Variables|/Script/Engine.CharacterMovementComponent|SetMaxWalkSpeed _charactermovement 2e+02)
      (Utilities|FlowControl|Sequence
        (:then_0
          (bind _height (Timeline|SetCapsuleHeight PlayFromStart)
            (:Update
              (Components|Capsule|SetCapsuleHalfHeight (Variables|Default|GetCapsuleComponent) (Math|Float|Lerp 9e+01 6e+01 _height) true)
              (Transformation|SetRelativeLocation (Variables|Character|GetMesh) (Math|Vector|MakeVector 0.0 0.0 (Math|Float|Lerp -89.0 -59.0 _height)) false false))))
        (:then_1
          (if (not (Variables|Default|GetSprinting))
            (bind _arm_length (Timeline|CrouchCamDistance PlayFromStart)
              (:Update
                (Variables|/Script/Engine.SpringArmComponent|SetTargetArmLength (Variables|Default|GetCameraBoom) (Math|Float|Lerp 4e+02 5e+02 _arm_length)))))))
      (else
        (bind _returnvalue_2 (Collision|SphereTraceByChannel _returnvalue (+ _returnvalue (* (Math|Vector|GetUpVector (Transformation|GetActorRotation)) 115.0)) 0.0 "TraceTypeQuery1" false 0 "None"))
        (if (not _returnvalue_2)
          (Variables|Default|SetCrouched false)
          (Variables|/Script/Engine.CharacterMovementComponent|SetMaxWalkSpeed _charactermovement 5e+02)
          (Utilities|FlowControl|Sequence
            (:then_0
              (Timeline|SetCapsuleHeight Reverse))
            (:then_1
              (if (not (Variables|Default|GetSprinting))
                (Timeline|CrouchCamDistance Reverse)))))))))

(event Input|EnhancedActionEvents|EnhancedInputActionIA_CameraSwitch
  (params (ActionValue :type Boolean) (ElapsedSeconds :type Float%20%28double-precision%29) (TriggeredSeconds :type Float%20%28double-precision%29) (InputAction :type Input%20Action%20Object%20Reference :default "/Game/ThirdPerson/Input/Actions/IA_CameraSwitch.IA_CameraSwitch"))
  ;[0.4025 1 0.1661 1 35] CAMERA SWITCH
  (:Started
    (Utilities|FlowControl|MultiGate false true -1
      (:Out%200
        ;;[1 1 1] FIRST PERSON CAMERA ON
        (Components|Activation|SetActive (Variables|Default|GetFPSCamera) true false)
        (Components|Activation|SetActive (Variables|Default|GetFollowCamera) false false)
        (Components|Activation|SetActive (Variables|Default|GetCombatCamera) false false)
        (Variables|Default|SetbUseControllerRotationYaw true))
      (:Out%201
        ;;[1 1 1] COMBAT THIRD PERSON CAMERA ON
        (Components|Activation|SetActive (Variables|Default|GetFPSCamera) false false)
        (Components|Activation|SetActive (Variables|Default|GetFollowCamera) false false)
        (Components|Activation|SetActive (Variables|Default|GetCombatCamera) true false)
        (Variables|Default|SetbUseControllerRotationYaw false))
      (:Out%202
        ;;[1 1 1] DEFAULT THIRD PERSON CAMERA ON
        (Components|Activation|SetActive (Variables|Default|GetFPSCamera) false false)
        (Components|Activation|SetActive (Variables|Default|GetFollowCamera) true false)
        (Components|Activation|SetActive (Variables|Default|GetCombatCamera) true false)
        (Variables|Default|SetbUseControllerRotationYaw false)))))

(event Input|EnhancedActionEvents|EnhancedInputActionIA_Sprint
  (params (ActionValue :type Boolean) (ElapsedSeconds :type Float%20%28double-precision%29) (TriggeredSeconds :type Float%20%28double-precision%29) (InputAction :type Input%20Action%20Object%20Reference :default "/Game/ThirdPerson/Input/Actions/IA_Sprint.IA_Sprint"))
  ;[1 1 1] Sprint
  (if (Variables|Default|GetSprinting)
    (Game|Feedback|ClientStartCameraShake (Game|GetPlayerController 0) "/Game/_DEV/CameraShake/Sprinting_CS.Sprinting_CS_C" 1.0 "CameraLocal" "0, 0, 0")))

(event Custom|BreakFirstLoop
  ;[1 1 1] HEIGHT OF OBSTACLE
  (Utilities|FlowControl|ForLoopwithBreak 0 4) ; enters at Break
)

(event Custom|ExecuteMotionWarping
  (bind _returnvalue (Transformation|GetActorRotation))
  (bind _mesh (Variables|Character|GetMesh))
  (bind _motionwarping (Variables|Default|GetMotionWarping))
  (bind _returnvalue_2 (Transformation|GetWorldLocation _mesh))
  (if (and (Variables|Default|GetCanWarp) (Math|Float|InRange(Float) (.z (Variables|Default|GetLandingSpot)) (- (.z _returnvalue_2) 5e+01) (+ (.z _returnvalue_2) 5e+01)))
    (Pawn|Components|CharacterMovement|SetMovementMode (Variables|Character|GetCharacterMovement) "MOVE_Flying" 0)
    (Collision|SetCollisionEnabled (Variables|Default|GetCapsuleComponent) "NoCollision")
    (Class|MotionWarpingComponent|AddorUpdateWarpTargetfromTransform _motionwarping "StartMotionWrap" (Math|Transform|MakeTransform (Variables|Default|GetStartSyncPoint) _returnvalue))
    (Class|MotionWarpingComponent|AddorUpdateWarpTargetfromTransform _motionwarping "LoopMotionWrap" (Math|Transform|MakeTransform (Variables|Default|GetDepthSyncPoint) _returnvalue))
    (Class|MotionWarpingComponent|AddorUpdateWarpTargetfromTransform _motionwarping "LandingMotionWrap" (Math|Transform|MakeTransform (Variables|Default|GetLandingSpot) _returnvalue))
    (Animation|Montage|PlayMontage (Variables|Character|GetMesh) "/Game/_NewDev/Animations/Vault/AM_VaultOver.AM_VaultOver"
      (:OnCompleted
        (Pawn|Components|CharacterMovement|SetMovementMode (Variables|Character|GetCharacterMovement) "MOVE_Walking" 0)
        (Collision|SetCollisionEnabled (Variables|Default|GetCapsuleComponent) "QueryAndPhysics")))))

(event Input|EnhancedActionEvents|EnhancedInputActionIA_Vault
  (params (ActionValue :type Boolean) (ElapsedSeconds :type Float%20%28double-precision%29) (TriggeredSeconds :type Float%20%28double-precision%29) (InputAction :type Input%20Action%20Object%20Reference :default "/Game/ThirdPerson/Input/Actions/IA_Vault.IA_Vault"))
  ;[1 1 1] HEIGHT OF OBSTACLE
  (bind _index (Utilities|FlowControl|ForLoopwithBreak 0 4)
    (:LoopBody
      (bind (_outhit _returnvalue) (Collision|SphereTraceByChannel (+ (Transformation|GetActorLocation) (Math|Vector|MakeVector 0.0 0.0 (* _index 30))) (+ (+ (Transformation|GetActorLocation) (Math|Vector|MakeVector 0.0 0.0 (* _index 30))) (* (Math|Vector|GetForwardVector (Transformation|GetActorRotation)) 1.8e+02)) 5.0 "TraceTypeQuery1" false 0 "None"))
      (if _returnvalue
        (CallFunction|BreakFirstLoop)
        ;[1 1 1] Depth of Obstacle
        (bind _index_2 (Utilities|FlowControl|ForLoopwithBreak 0 5 :!label _label)
          (:LoopBody
            (bind (_outhit_2 _returnvalue_2) (Collision|SphereTraceByChannel (+ (+ (.Location (Collision|BreakHitResult _outhit)) "0.000000,0.000000,90.000000") (* (Math|Vector|GetForwardVector (Transformation|GetActorRotation)) (* _index_2 50))) (- (+ (+ (.Location (Collision|BreakHitResult _outhit)) "0.000000,0.000000,90.000000") (* (Math|Vector|GetForwardVector (Transformation|GetActorRotation)) (* _index_2 50))) "0.000000,0.000000,100.000000") 6.0 "TraceTypeQuery1" false 0 "None"))
            (if _returnvalue_2
              (if (.bInitialOverlap (Collision|BreakHitResult _outhit_2))
                (Variables|Default|SetCanWarp false)
                (Variables|Default|SetLandingSpot "0.000000,0.000000,2000.000000")
                (goto _label Break)
                (else
                  (Utilities|FlowControl|Sequence
                    (:then_0
                      (if (== _index_2 0)
                        (Variables|Default|SetStartSyncPoint (.Location (Collision|BreakHitResult _outhit_2)))))
                    (:then_1
                      (Variables|Default|SetDepthSyncPoint (.Location (Collision|BreakHitResult _outhit_2)))
                      (Variables|Default|SetCanWarp true)))))
              (else
                (bind (_outhit_3 _returnvalue_3) (Collision|LineTraceByChannel (+ (.TraceStart (Collision|BreakHitResult _outhit_2)) (* (Math|Vector|GetForwardVector (Transformation|GetActorRotation)) 75.0)) (- (+ (.TraceStart (Collision|BreakHitResult _outhit_2)) (* (Math|Vector|GetForwardVector (Transformation|GetActorRotation)) 75.0)) "0.000000,0.000000,1000.000000") "TraceTypeQuery1" false 0 "ForDuration"))
                (if _returnvalue_3
                  (Variables|Default|SetLandingSpot (.Location (Collision|BreakHitResult _outhit_3)))
                  (goto _label Break)))))
          (:Completed
            (CallFunction|ExecuteMotionWarping)))))))

(event Input|EnhancedActionEvents|EnhancedInputActionIA_Jump
  (params (ActionValue :type Boolean) (ElapsedSeconds :type Float%20%28double-precision%29) (TriggeredSeconds :type Float%20%28double-precision%29) (InputAction :type Input%20Action%20Object%20Reference :default "/Game/ThirdPerson/Input/Actions/IA_Jump.IA_Jump"))
  (:Started
    (if (Character|CanJump)
      (bind _canclimb_vault (Default|MantleGroundCheck (Variables|Default|GetMantleSystem)))
      (if (not _canclimb_vault)
        (Character|Jump)))))

(event Input|EnhancedActionEvents|EnhancedInputActionIA_Slide
  (params (ActionValue :type Boolean) (ElapsedSeconds :type Float%20%28double-precision%29) (TriggeredSeconds :type Float%20%28double-precision%29) (InputAction :type Input%20Action%20Object%20Reference :default "/Game/ThirdPerson/Input/Actions/IA_Slide.IA_Slide"))
  (:Started
    (if (> (Math|Vector|VectorLength (Variables|/Script/Engine.MovementComponent|GetVelocity (Variables|Character|GetCharacterMovement))) 2e+02)
      (Variables|Default|SetIsSliding true)
      (bind (_direction _setcapsuleheight _cameralocation _cameraheight) (Timeline|Timeline PlayFromStart)
        (:Update
          (Utilities|FlowControl|Sequence
            (:then_0
              (Components|Capsule|SetCapsuleHalfHeight (Variables|Default|GetCapsuleComponent) _setcapsuleheight true))
            (:then_1
              (Transformation|SetRelativeLocation (Variables|Character|GetMesh) (Math|Vector|MakeVector 0.0 0.0 _cameralocation) false false)))))))
  (:Canceled
    (if (Variables|Default|GetIsSliding) :!label _label
      (Variables|Default|SetIsSliding false)
      (Timeline|Timeline Reverse)))
  (:Completed
    (goto _label)))

(fn ConstructionScript
  (|CallParentFunction))